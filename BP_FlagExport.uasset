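; Export utility that dumps an AAS capture-zone layout as JSON on BeginPlay, including two map corner positions.
; It walks the AAS initializer's DesignOutgoingLinks, recording each flag's name, initial team, location, child-component bounds and next flag, plus the final end node.
; Helper functions hand-build the JSON through string appends.
; Output splits it into lines, tracks brace depth for indentation and emits each via PrintString.
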(event `self.ReceiveBeginPlay`
  (bind _designoutgoinglinks (`SQGraphInitializerComponent.DesignOutgoingLinks` (`self.GetComponentByClass` (`self.AASZones`) "/Script/Squad.SQGraphAASInitializerComponent")))
  (bind _json_out (`self.JsonVector` "corner_1" (`SceneComponent.K2_GetComponentLocation` (`/Game/Blueprints/Placeable/BP_CornerMarker.DefaultSceneRoot` (`self.Corner1`)))))
  (bind _json_out_2 (`self.JsonVector` "corner_2" (`SceneComponent.K2_GetComponentLocation` (`/Game/Blueprints/Placeable/BP_CornerMarker.DefaultSceneRoot` (`self.Corner2`)))))
  (set `self.JsonOut` (`KismetStringLibrary.Concat_StrStr` "{\\n" _json_out _json_out_2 "\"flags\" : {\\n"))
  (for (_array_element _array_index) _designoutgoinglinks
    (bind (_nodea _nodeb) (break `SQDesignLink` _array_element))
    (bind _flagjsonout (`self.JsonFlag` _nodea _nodeb))
    (set `self.JsonOut` (`KismetStringLibrary.Concat_StrStr` (`self.JsonOut`) _flagjsonout))
    (`/Engine/EditorBlueprintResources/StandardMacros.CompareInt` _array_index (- (`KismetArrayLibrary.Array_Length` _designoutgoinglinks) 1)
      (:`==`
        (bind _flagjsonout_2 (`self.JsonFlag` _nodeb))
        (set `self.JsonOut` (`KismetStringLibrary.Concat_StrStr` (`self.JsonOut`) _flagjsonout_2)))))
  (`self.Output` (`KismetStringLibrary.Concat_StrStr` (`self.JsonOut`) "}\\n" "}")))

(fn `JsonBounds`
  (params (Root :type "SceneComponent Object Reference"))
  (returns (JsonOut :type String))
  (locals (`Json Out Temp` :type String))
  (bind _children (`SceneComponent.GetChildrenComponents` Root false))
  (set `local.Json Out Temp` "\"bounds\" : {\\n")
  (for (_array_element _array_index) _children
    (bind (_origin _boxextent) (`KismetSystemLibrary.GetComponentBounds` _array_element))
    (bind _json_out (`self.JsonVector` "origin" _origin))
    (bind _json_out_2 (`self.JsonVector` "box_extent" _boxextent))
    (bind _output (`self.JsonString` "rotation" (`KismetStringLibrary.Conv_DoubleToString` (.yaw (`SceneComponent.K2_GetComponentRotation` _array_element)))))
    (`/Engine/EditorBlueprintResources/StandardMacros.CompareInt` _array_index (- (`KismetArrayLibrary.Array_Length` _children) 1)
      (:`>`
        (bind _returnvalue (`KismetStringLibrary.Concat_StrStr` (`local.Json Out Temp`) "\"" (`KismetSystemLibrary.GetObjectName` _array_element) "\" : {\\n" _json_out _json_out_2 (`KismetStringLibrary.Replace` _output ",")))
        (set `local.Json Out Temp` (`KismetStringLibrary.Concat_StrStr` _returnvalue "},\\n") :!label _label))
      (:`==`
        (set `local.Json Out Temp` (`KismetStringLibrary.Concat_StrStr` _returnvalue "}\\n")))
      (:`<`
        (goto _label))))
  (set `local.Json Out Temp` (`KismetStringLibrary.Concat_StrStr` (`local.Json Out Temp`) "},\\n"))
  (return (`local.Json Out Temp`)))

(fn `JsonFlag`
  (params (Zone :type "Actor Object Reference") (NextZone :type "Actor Object Reference"))
  (returns (FlagJsonOut :type String))
  (bind _returnvalue (`self.GetComponentByClass` Zone "/Script/Squad.SQCaptureZoneComponent"))
  (bind _rootcomponent (`Actor.RootComponent` Zone))
  (bind _output (`self.JsonString` "display_name" (`KismetTextLibrary.Conv_TextToString` (`SQCaptureZoneComponent.FlagName` _returnvalue))))
  (bind _output_2 (`self.JsonString` "initial_team" (`KismetStringLibrary.Conv_ByteToString` (`SQCaptureZoneComponent.InitialTeam` _returnvalue))))
  (bind _json_out (`self.JsonVector` "location" (`SceneComponent.K2_GetComponentLocation` _rootcomponent)))
  (bind _jsonout (`self.JsonBounds` _rootcomponent))
  (bind _output_3 (`self.JsonString` "next_flag" (`KismetSystemLibrary.GetObjectName` NextZone)))
  (return (`KismetStringLibrary.Concat_StrStr` "\"" (`KismetSystemLibrary.GetObjectName` Zone) "\"" " : {\\n" _output _output_2 _json_out _jsonout (`KismetStringLibrary.Replace` _output_3 ",") "},\\n")))

(fn `JsonString`
  (params (Name :type String) (Value :type String))
  (returns (Output :type String))
  (return (`KismetStringLibrary.Concat_StrStr` "\"" Name "\" : \"" Value "\",\\n")))

(fn `JsonVector`
  (params (Name :type String) (`Vector In` :type "Vector Structure"))
  (returns (`Json Out` :type String))
  (bind _output (`self.JsonString` "x" (`KismetStringLibrary.Conv_DoubleToString` (.x `Vector In`))))
  (bind _output_2 (`self.JsonString` "y" (`KismetStringLibrary.Conv_DoubleToString` (.y `Vector In`))))
  (bind _output_3 (`self.JsonString` "z" (`KismetStringLibrary.Conv_DoubleToString` (.z `Vector In`))))
  (return (`KismetStringLibrary.Concat_StrStr` "\"" Name "\" : {\\n" _output _output_2 (`KismetStringLibrary.Replace` _output_3 ",") "},\\n")))

(fn `Output`
  (params (Output :type String))
  (locals (OutString :type String) (OutArray :type "Array of String") (Indent :type Integer) (IndentString :type String :default "Hello"))
  (bind _outarray (`local.OutArray`))
  (bind (_lefts _rights _returnvalue) (`KismetStringLibrary.Split` (`local.OutString`) "\\n" "CaseSensitive"))
  (set `local.OutString` Output)
  (while _returnvalue
    (`KismetArrayLibrary.Array_Add` _outarray _lefts)
    (bind _output_get (set `local.OutString` _rights)))
  (`KismetArrayLibrary.Array_Add` _outarray _output_get)
  (for _array_element _outarray
    (`/Engine/EditorBlueprintResources/StandardMacros.CompareInt` (`KismetStringLibrary.FindSubstring` _array_element "}") -1
      (:`>`
        (`/Engine/EditorBlueprintResources/StandardMacros.DecrementInt` (`local.Indent`) :!label _label
          (:`  `
            _)))
      (:`==`
        _)
      (:`<`
        (goto _label)))
    (set `local.IndentString` "")
    (for _ (range (+ (`local.Indent`) 1))
      (set `local.IndentString` (`KismetStringLibrary.Concat_StrStr` (`local.IndentString`) "  ")))
    (`KismetSystemLibrary.PrintString` (`KismetStringLibrary.Concat_StrStr` (`local.IndentString`) _array_element))
    (`/Engine/EditorBlueprintResources/StandardMacros.CompareInt` (`KismetStringLibrary.FindSubstring` _array_element "{") -1
      (:`>`
        _)
      (:`<`
        _))
    (`/Engine/EditorBlueprintResources/StandardMacros.IncrementInt` (`local.Indent`))))

(fn `UserConstructionScript`)